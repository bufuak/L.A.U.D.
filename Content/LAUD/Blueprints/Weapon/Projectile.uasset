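; Projectile actor for VR weapon fire that deals damage on overlap and can come from either an enemy or the player.
; Its sphere collision ignores the VR pawn unless the shot is flagged as enemy fire, then sends a damage message to the hit actor.
; Physics-simulating components also get an impulse along the projectile's velocity, stronger for non-enemy shots.
; The projectile destroys itself only in that physics case.
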(event OnComponentBeginOverlap(SphereCollision)
  (params (OverlappedComponent :type Primitive%20Component%20Object%20Reference) (OtherActor :type Actor%20Object%20Reference) (OtherComp :type Primitive%20Component%20Object%20Reference) (OtherBodyIndex :type Integer) (bFromSweep :type Boolean) (SweepResult :type Hit%20Result%20Structure%20%28by%20ref%29))
  (Utilities|Casting|CastToVRPawn OtherActor
    (:then
      (if (Variables|Default|GetShootByEnemy)
        (Class|BPIDamageable|ApplyDamage(Message) OtherActor 1e+01 :!label _label)
        (if (Physics|IsSimulatingPhysics OtherComp "None")
          (Physics|AddImpulse OtherComp (* (Variables|/Script/Engine.MovementComponent|GetVelocity (Variables|Default|GetProjectileMovement)) (Math|Float|SelectFloat 1.0 5.0 (Variables|Default|GetShootByEnemy))) "None" false)
          ;[0.03434 0.03434 0.03434] Destroy the projectile
          (Actor|DestroyActor))))
    (:CastFailed
      (goto _label))))

(fn ConstructionScript)