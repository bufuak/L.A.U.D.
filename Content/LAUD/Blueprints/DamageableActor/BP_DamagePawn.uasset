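; BP_DamagePawn is a damageable pawn that tracks health and destroys itself when that health runs out.
; Health starts at MaxHealth on BeginPlay, and ApplyDamage subtracts from it, clamped between zero and the maximum.
; Reaching zero fires DeadHandle through a DoOnce so death runs a single time, and DeadHandle destroys the actor.
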(event Custom|DeadHandle
  (Actor|DestroyActor))

(event EventBeginPlay
  (|CallParentFunction)
  (Variables|Damage|SetHealth (Variables|Damage|GetMaxHealth)))

(event Collision|EventActorBeginOverlap
  (params (OtherActor :type Actor%20Object%20Reference)))

(event EventTick
  (params (DeltaSeconds :type Float%20%28single-precision%29))
  (|CallParentFunction DeltaSeconds))

(event EventApplyDamage
  (params (Damage :type Float%20%28single-precision%29))
  (bind _output_get (Variables|Damage|SetHealth (Math|Float|Clamp(Float) (- (Variables|Damage|GetHealth) Damage) 0.0 (Variables|Damage|GetMaxHealth))))
  (if (== _output_get 0.0)
    (Utilities|FlowControl|DoOnce false
      (:Completed
        (CallFunction|DeadHandle)))))

(fn ConstructionScript)