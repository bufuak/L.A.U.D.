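; Behavior tree service that feeds enemy AI values into the blackboard.
; Each tick it writes the first player pawn's location to the player location key.
; A DoOnce then casts the controlled pawn to BP_EnemyBase and stores its melee flag and current location a single time, printing that location to screen.
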(event EventReceiveActivationAI
  (params (OwnerController :type AI%20Controller%20Object%20Reference) (ControlledPawn :type Pawn%20Object%20Reference)))

(event EventReceiveTickAI
  (params (OwnerController :type AI%20Controller%20Object%20Reference) (ControlledPawn :type Pawn%20Object%20Reference) (DeltaSeconds :type Float%20%28single-precision%29))
  (bind _returnvalue (Transformation|GetActorLocation ControlledPawn))
  (AI|BehaviorTree|SetBlackboardValueasVector (Variables|Default|GetPlayerLocationKey) (Transformation|GetActorLocation (Game|Player|GetPlayerPawn 0)))
  (Utilities|FlowControl|DoOnce false
    (:Completed
      (bind _asbp_enemy_base (Utilities|Casting|CastToBP_EnemyBase ControlledPawn))
      (Class|BTFunctionLibrary|SetBlackboardValueasBool (Variables|Default|GetMeleeKey) (Variables|/Game/LAUD/Blueprints/Enemy/BP_EnemyBase.BP_EnemyBase_C|GetbIsMelee _asbp_enemy_base))
      (AI|BehaviorTree|SetBlackboardValueasVector (Variables|Default|GetActorLocationKey) _returnvalue)
      (Development|PrintString (Utilities|String|ToString(Vector) _returnvalue)))))