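; Behavior tree task that makes an enemy derived from BP_EnemyBase fire one projectile.
; On execute it casts the controlled pawn, spawns the projectile at the weapon's Muzzle socket transform flagged as shot by an enemy, then finishes successfully at once.
; Shot direction comes from the socket alone, as the player-relative vector math is left unconnected.
; A failed cast never calls FinishExecute.
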(event EventReceiveExecuteAI
  (params (OwnerController :type AI%20Controller%20Object%20Reference) (ControlledPawn :type Pawn%20Object%20Reference))
  (bind _asbp_enemy_base (Utilities|Casting|CastToBP_EnemyBase ControlledPawn))
  (Game|SpawnActorfromClass "/Game/LAUD/Blueprints/Weapon/Projectile.Projectile_C" (Transformation|GetSocketTransform (Variables|/Game/LAUD/Blueprints/Enemy/BP_EnemyBase.BP_EnemyBase_C|GetWeapon _asbp_enemy_base) "Muzzle" "RTS_World") "Undefined" 0 true 0)
  (AI|BehaviorTree|FinishExecute true))