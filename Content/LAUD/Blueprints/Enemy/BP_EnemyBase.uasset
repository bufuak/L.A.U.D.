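; Base enemy Blueprint with melee and ranged variants selected by IsMelee, handling appearance setup and death.
; The construction script applies a dynamic material to the mesh, then removes the weapon for melee or attaches it to the right-hand socket.
; DeadHandle drives the material's Apperance parameter through a timeline before destroying the actor.
; Ranged enemies first swap their weapon component for a spawned Pistol actor.
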(event EventBeginPlay
  (|CallParentFunction))

(event Collision|EventActorBeginOverlap
  (params (OtherActor :type Actor%20Object%20Reference)))

(event EventTick
  (params (DeltaSeconds :type Float%20%28single-precision%29)))

(event EventDeadHandle
  (if (Variables|Default|GetbIsMelee)
    (bind _newtrack_0 (Timeline|Timeline_0 PlayFromStart)
      (:Update
        (Rendering|Material|SetScalarParameterValue (Variables|Default|GetMaterialInstance) "Apperance" _newtrack_0 :!class /Script/Engine.MaterialInstanceDynamic))
      (:Finished
        (Actor|DestroyActor)))
    (else
      (Components|DestroyComponent (Variables|Default|GetWeapon))
      (Game|SpawnActorfromClass "/Game/LAUD/Blueprints/Weapon/Pistol.Pistol_C" (Transformation|GetWorldTransform (Variables|Default|GetScene)) "Undefined" 0 true 0)
      (Timeline|Timeline_0 PlayFromStart))))

(fn ConstructionScript
  (bind _returnvalue (Rendering|Material|CreateDynamicMaterialInstance "/Engine/Tutorial/SubEditors/TutorialAssets/Character/TutorialTPP_Mat_Inst.TutorialTPP_Mat_Inst" "None" "None" :!class /Script/Engine.KismetMaterialLibrary))
  (bind _output_get (Variables|Default|SetMaterialInstance _returnvalue))
  (Rendering|Material|SetMaterial (Variables|Character|GetMesh) 0 _output_get)
  (if (Variables|Default|GetbIsMelee)
    (Components|DestroyComponent (Variables|Default|GetWeapon))
    (else
      (Transformation|AttachComponentToComponent (Variables|Default|GetWeapon) (Variables|Character|GetMesh) "hand_r" "KeepRelative" "KeepRelative" "KeepRelative" true))))