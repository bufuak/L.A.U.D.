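; Behavior tree decorator that passes when an enemy AI pawn has line of sight to the player.
; It requires the pawn to be within a fixed range of the PlayerLocation blackboard value, then traces from that location, at a hardcoded world height, to the pawn.
; The trace tests only WorldStatic objects, so the condition fails when static geometry blocks it or the player is out of range.
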(fn PerformConditionCheckAI
  (params (OwnerController :type AI%20Controller%20Object%20Reference) (ControlledPawn :type Pawn%20Object%20Reference))
  (bind _returnvalue (Transformation|GetActorLocation ControlledPawn))
  (bind _playerlocation (Variables|Default|GetPlayerLocation))
  (bind _returnvalue_2 (Class|BTFunctionLibrary|GetBlackboardValueasVector _playerlocation))
  (if (< (Math|Vector|VectorLength (- _returnvalue (Class|BTFunctionLibrary|GetBlackboardValueasVector _playerlocation))) 2e+03)
    (bind _returnvalue_3 (Collision|LineTraceForObjects (Math|Vector|MakeVector (.x _returnvalue_2) (.y _returnvalue_2) 1.6e+02) _returnvalue (Utilities|Array|MakeArray "ObjectTypeQuery1") false 0 "None" false))
    (if _returnvalue_3
      (return false)
      (else
        (return true)))
    (else
      (return false))))